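; Blueprint function library of helpers for a Redux-style to-do list state system.
; Action creators build typed Add Todo, Toggle Todo and Set Visibility Filter actions through CreateAction and fill in their fields.
; GetStore fetches the store from MyHUD on player 0's controller, and Subscribe uses it to bind a callback to the store's state-change event.
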(fn CreateSetVisibilityFilterAction
  (params (Filter :type String))
  (bind _asset_visibility_filter_action (Utilities|Casting|CastToSetVisibilityFilterAction (Class|ReduxBlueprintFunctionLibrary|CreateAction "/Script/Todos.SetVisibilityFilterAction")))
  (Variables|/Script/Todos.SetVisibilityFilterAction|SetFilter _asset_visibility_filter_action Filter)
  (return _asset_visibility_filter_action))

(fn Subscribe
  (params (이벤트 :type Delegate%20%28by%20ref%29))
  (bind _store (CallFunction|GetStore))
  (EventDispatchers|BindEventtoOnStateChanged _store 이벤트))

(fn CreateAddTodoAction
  (params (Id :type Integer) (Text :type Text))
  (bind _asadd_todo_action (Utilities|Casting|CastToAddTodoAction (Class|ReduxBlueprintFunctionLibrary|CreateAction "/Script/Todos.AddTodoAction")))
  (Variables|/Script/Todos.AddTodoAction|SetId _asadd_todo_action Id)
  (Variables|/Script/Todos.AddTodoAction|SetText _asadd_todo_action Text)
  (return _asadd_todo_action))

(fn CreateToggleTodoAction
  (params (Id :type Integer))
  (bind _astoggle_todo_action (Utilities|Casting|CastToToggleTodoAction (Class|ReduxBlueprintFunctionLibrary|CreateAction "/Script/Todos.ToggleTodoAction")))
  (Variables|/Script/Todos.ToggleTodoAction|SetId _astoggle_todo_action Id)
  (return _astoggle_todo_action))

(fn GetStore
  (bind _asmy_hud (Utilities|Casting|CastToMyHUD (HUD|GetHUD (Game|GetPlayerController 0))))
  (bind _returnvalue (Class|MyHUD|GetStore _asmy_hud))
  (return _returnvalue))